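; Interactive storybook actor whose pages flip forward and back on mouse or shoulder-button input while open, with page-turn sounds.
; Entering or leaving its trigger shows or hides the key prompt on a StorybookUI widget created at BeginPlay, with open/close sounds.
; Selecting a page plays a one-time appear effect, then activates the level portal when it finishes.
; The construction script sets the book's material from Mine and Canyon completion in the game instance.
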(event `Key|Gamepad_RightShoulder`
  (params (Key :type "Key Structure"))
  (:`Pressed`
    (if (`self.m_bIsOpen`) :!label _label
      (`GameplayStatics.PlaySound2D` "/Game/Sound/SFX/Book_and_Menu/Book_Change_Page_003.Book_Change_Page_003" 1.0 1.0 0.0 null null)
      (`self.FlipPageForward`))))

(event `Key|RightMouseButton`
  (params (Key :type "Key Structure"))
  (:`Pressed`
    (goto _label)))

(event `Key|LeftMouseButton`
  (params (Key :type "Key Structure"))
  (:`Pressed`
    (if (`self.m_bIsOpen`) :!label _label_2
      (`GameplayStatics.PlaySound2D` "/Game/Sound/SFX/Book_and_Menu/Book_Change_Page_002.Book_Change_Page_002" 1.0 1.0 0.0 null null)
      (`self.FlipPageBack`))))

(event `Key|Gamepad_LeftShoulder`
  (params (Key :type "Key Structure"))
  (:`Pressed`
    (goto _label_2)))

(event `self.OnPageSelect`
  (params (PageForwardFlipCount :type Integer))
  (bind _appeareffect (`self.AppearEffect`))
  (if (not (`self.bSelected`))
    (set `self.bSelected` true)
    (add `/Game/LevelAssets/Library/VFX/PortalAppear/AppearalEffect.OnAnimationFinished` _appeareffect (delegate `OnPortalAnimEnd`))
    (`/Game/LevelAssets/Library/VFX/PortalAppear/AppearalEffect.OnPlayAppearAnimation` _appeareffect)))

(event `OnPortalAnimEnd`
  (`/Game/LevelAssets/Library/Actors/AetherPortal.ActivatePortal` (`self.AetherPortal`)) ; Only opens level portal
)

(event `self.m_pTrigger.OnComponentBeginOverlap`
  (params (OverlappedComponent :type "PrimitiveComponent Object Reference") (OtherActor :type "Actor Object Reference") (OtherComp :type "PrimitiveComponent Object Reference") (OtherBodyIndex :type Integer) (bFromSweep :type Boolean) (SweepResult :type "HitResult Structure (by ref)"))
  (bind _keywidget (`/Game/UI/Keys/IKeyWidget.GetKeyWidget` (`self.BookUI`)))
  (`/Game/UI/Keys/KeyWidgetBase.ShowWidget` _keywidget)
  (`GameplayStatics.PlaySound2D` "/Game/Sound/SFX/Book_and_Menu/Book_Open_001.Book_Open_001" 1.0 1.0 0.0 null null))

(event `self.m_pTrigger.OnComponentEndOverlap`
  (params (OverlappedComponent :type "PrimitiveComponent Object Reference") (OtherActor :type "Actor Object Reference") (OtherComp :type "PrimitiveComponent Object Reference") (OtherBodyIndex :type Integer))
  (bind _keywidget (`/Game/UI/Keys/IKeyWidget.GetKeyWidget` (`self.BookUI`)))
  (`/Game/UI/Keys/KeyWidgetBase.HideWidget` _keywidget)
  (`GameplayStatics.PlaySound2D` "/Game/Sound/SFX/Book_and_Menu/Book_Close_001.Book_Close_001" 1.0 1.0 0.0 null null))

(event `self.ReceiveBeginPlay`
  (bind _returnvalue (`|CreateWidget` "/Game/LevelAssets/Library/Actors/Storybook/StorybookUI.StorybookUI_C"))
  (`UserWidget.AddToViewport` _returnvalue 0)
  (set `self.BookUI` _returnvalue))

(fn `UserConstructionScript`
  (bind _m_pskelmesh (`self.m_pSkelMesh`))
  (bind _asastgame_instance (cast `ASTGameInstance` (`GameplayStatics.GetGameInstance`)))
  (if (`ASTGameInstance.IsMineLevelDone` _asastgame_instance)
    (if (`ASTGameInstance.IsCanyonLevelDone` _asastgame_instance)
      (`PrimitiveComponent.SetMaterial` _m_pskelmesh 0 "/Game/LevelAssets/Library/Actors/Storybook/Storybook03_M.Storybook03_M")
      (else
        (`PrimitiveComponent.SetMaterial` _m_pskelmesh 0 "/Game/LevelAssets/Library/Actors/Storybook/Storybook02_M_Inst.Storybook02_M_Inst")))))