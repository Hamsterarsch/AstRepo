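; Canyon level prop that builds a chain along an editable spline from a repeated link mesh.
; The construction script divides spline length by Spacing and adds two static mesh components per step, oriented to the spline.
; The second link sits half a step back with Rotation added to its roll, producing alternating links.
; Components use manual attachment with world-space transforms, and the event graph has no active logic.
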(fn `UserConstructionScript`
  (bind _spline (`self.Spline`))
  (bind _spline_2 (`self.Spline`))
  (bind _spacing (`self.Spacing`))
  (bind _mesh (`self.mesh`))
  (for _index (range 1 (+ (`.ReturnValue` (`KismetMathLibrary.FMod` (`SplineComponent.GetSplineLength` (`self.Spline`)) _spacing)) 1))
    (bind _returnvalue (* _index _spacing))
    (bind _returnvalue_2 (`AddComponent|NODE_AddStaticMeshComponent-1` :`bManualAttachment` true :`RelativeTransform` (`KismetMathLibrary.MakeTransform` (`SplineComponent.GetLocationAtDistanceAlongSpline` _spline_2 _returnvalue "World") (`SplineComponent.GetRotationAtDistanceAlongSpline` _spline_2 _returnvalue "World"))))
    (`StaticMeshComponent.SetStaticMesh` _returnvalue_2 _mesh)
    (bind _returnvalue_3 (- _returnvalue (/ _spacing 2.0)))
    (bind _returnvalue_4 (`AddComponent|NODE_AddStaticMeshComponent-0` :`bManualAttachment` true :`RelativeTransform` (`KismetMathLibrary.MakeTransform` (`SplineComponent.GetLocationAtDistanceAlongSpline` _spline _returnvalue_3 "World") (`KismetMathLibrary.MakeRotator` (+ (.roll (`SplineComponent.GetRotationAtDistanceAlongSpline` _spline _returnvalue_3 "World")) (`self.Rotation`)) (.pitch (`SplineComponent.GetRotationAtDistanceAlongSpline` _spline _returnvalue_3 "World")) (.yaw (`SplineComponent.GetRotationAtDistanceAlongSpline` _spline _returnvalue_3 "World"))))))
    (`StaticMeshComponent.SetStaticMesh` _returnvalue_4 _mesh)))