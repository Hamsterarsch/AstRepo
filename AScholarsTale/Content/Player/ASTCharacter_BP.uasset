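; Player character Blueprint that adds sound, camera and effect feedback to movement, plus gamepad debug controls.
; Jump, land and movement input play camera anims or shakes, a timeline bobs the camera, and the custom Gliding mode toggles particles and looping audio.
; A downward trace picks surface-based landing sounds and random footsteps loaded from object libraries.
; Debug buttons toggle flying, open levels and scale post-process gamma/gain, with D-pad up/down doubling as flight altitude.
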(event `Key|Gamepad_DPad_Up`
  (params (Key :type "Key Structure"))
  (bind _m_pcamera (`self.m_pCamera`))
  (bind ((`ColorGamma` _colorgamma) (`ColorGain` _colorgain)) (break `PostProcessSettings` (`CameraComponent.PostProcessSettings` _m_pcamera)))
  ;[1 1 1] Post Brighten
  (:`Pressed`
    (bind _outvec (`self.ScaleVec4` _colorgamma 1.1))
    (set `CameraComponent.PostProcessSettings` (make `PostProcessSettings` :`ColorGamma` _outvec :`ColorGain` _colorgain) _m_pcamera)))

(event `Key|Gamepad_DPad_Down`
  (params (Key :type "Key Structure"))
  (bind _m_pcamera (`self.m_pCamera`))
  (bind ((`ColorGamma` _colorgamma) (`ColorGain` _colorgain)) (break `PostProcessSettings` (`CameraComponent.PostProcessSettings` _m_pcamera)))
  ;[1 1 1] Post Brighten
  (:`Pressed`
    (bind _outvec (`self.ScaleVec4` _colorgamma 0.9))
    (set `CameraComponent.PostProcessSettings` (make `PostProcessSettings` :`ColorGamma` _outvec :`ColorGain` _colorgain) _m_pcamera)))

(event `Key|Gamepad_DPad_Left`
  (params (Key :type "Key Structure"))
  (bind _m_pcamera (`self.m_pCamera`))
  (bind ((`ColorGamma` _colorgamma) (`ColorGain` _colorgain)) (break `PostProcessSettings` (`CameraComponent.PostProcessSettings` _m_pcamera)))
  ;[1 1 1] Post Brighten
  (:`Pressed`
    (bind _outvec (`self.ScaleVec4` _colorgain 1.1))
    (set `CameraComponent.PostProcessSettings` (make `PostProcessSettings` :`ColorGamma` _colorgamma :`ColorGain` _outvec) _m_pcamera)))

(event `Key|Gamepad_DPad_Right`
  (params (Key :type "Key Structure"))
  (bind _m_pcamera (`self.m_pCamera`))
  (bind ((`ColorGamma` _colorgamma) (`ColorGain` _colorgain)) (break `PostProcessSettings` (`CameraComponent.PostProcessSettings` _m_pcamera)))
  ;[1 1 1] Post Brighten
  (:`Pressed`
    (bind _outvec (`self.ScaleVec4` _colorgain 0.9))
    (set `CameraComponent.PostProcessSettings` (make `PostProcessSettings` :`ColorGamma` _colorgamma :`ColorGain` _outvec) _m_pcamera)))

(event `Key|Gamepad_LeftShoulder`
  (params (Key :type "Key Structure"))
  (bind _charactermovement (`self.CharacterMovement`))
  ;[1 1 1] Cheat
  (:`Pressed`
    (switch `EMovementMode` (`CharacterMovementComponent.MovementMode` (`self.CharacterMovement`))
      (:`MOVE_None`
        (`CharacterMovementComponent.SetMovementMode` _charactermovement "MOVE_Flying" 0 :!label _label)
        (set `self.bIsFlying` true))
      (:`MOVE_Walking`
        (goto _label))
      (:`MOVE_Falling`
        (goto _label))
      (:`MOVE_Swimming`
        (goto _label))
      (:`MOVE_Flying`
        (`CharacterMovementComponent.SetMovementMode` _charactermovement "MOVE_Walking" 0)
        (set `self.bIsFlying` false))
      (:`MOVE_Custom`
        (goto _label)))))

(event `Key|Gamepad_Special_Left`
  (params (Key :type "Key Structure"))
  ;[1 1 1] Cheat
  (:`Pressed`
    (`GameplayStatics.OpenLevel` "Library")))

(event `Key|Gamepad_Special_Right`
  (params (Key :type "Key Structure"))
  ;[1 1 1] Cheat
  (:`Pressed`
    (`GameplayStatics.OpenLevel` "Canyon")))

(event `Key|Gamepad_DPad_Up`
  (params (Key :type "Key Structure"))
  (bind _bisflying (`self.bIsFlying`))
  ;[1 1 1] Cheat
  (:`Pressed`
    (if _bisflying
      (set `self.bHeldUp` true)))
  (:`Released`
    (if _bisflying
      (set `self.bHeldUp` false))))

(event `Key|Gamepad_DPad_Down`
  (params (Key :type "Key Structure"))
  (bind _bisflying (`self.bIsFlying`))
  ;[1 1 1] Cheat
  (:`Pressed`
    (if _bisflying
      (set `self.bHeldDown` true)))
  (:`Released`
    (if _bisflying
      (set `self.bHeldDown` false))))

(event `self.ReceiveTick`
  (params (DeltaSeconds :type "Float (single-precision)"))
  (bind _charactermovement (`self.CharacterMovement`))
  ;[1 1 1] Cheat
  (`|ExecutionSequence`
    (:`then_0`
      (if (`self.bHeldUp`)
        (`PawnMovementComponent.AddInputVector` _charactermovement (0.0 0.0 1.0) false)))
    (:`then_1`
      (if (`self.bHeldDown`)
        (`PawnMovementComponent.AddInputVector` _charactermovement (0.0 0.0 -1.0) false)))))

(event `self.K2_OnMovementModeChanged`
  (params (PrevMovementMode :type "EMovementMode Enum" :default "MOVE_None") (NewMovementMode :type "EMovementMode Enum" :default "MOVE_None") (PrevCustomMode :type Byte) (NewCustomMode :type Byte))
  (bind _audioglidingloop (`self.AudioGlidingLoop`))
  ;[1 1 1] Movement mode effects
  (`|ExecutionSequence`
    (:`then_0`
      ;;[1 1 1] Previous mode handling
      (switch `EMovementMode` PrevMovementMode
        (:`MOVE_Custom`
          (switch `EASTMovementMode` (cast `EASTMovementMode` PrevCustomMode)
            (:`Gliding`
              (`ActorComponent.Deactivate` (`self.GlidingEffect_PS`))
              (`/Engine/EditorBlueprintResources/StandardMacros.IsValid` _audioglidingloop
                (:`Is Valid`
                  (`AudioComponent.FadeOut` _audioglidingloop 0.5 0.0))))))))
    (:`then_1`
      ;;[1 1 1] New mode handling
      (switch `EMovementMode` NewMovementMode
        (:`MOVE_Custom`
          (switch `EASTMovementMode` (cast `EASTMovementMode` NewCustomMode)
            (:`Gliding`
              (`ActorComponent.Activate` (`self.GlidingEffect_PS`) false)
              (`/Engine/EditorBlueprintResources/StandardMacros.IsValid` (`self.AudioGlidingLoop`)
                (:`Is Valid`
                  _)
                (:`Is Not Valid`
                  (bind _returnvalue (`GameplayStatics.SpawnSound2D` "/Game/Sound/SFX/Player/player_glider_loop.player_glider_loop" 1.0 1.0 0.0 null))
                  (set `self.AudioGlidingLoop` _returnvalue)))
              (`AudioComponent.FadeIn` (`self.AudioGlidingLoop`) 1.0 1.0 0.0))))))))

(event `self.ReceiveBeginPlay`
  ;[1 1 1] Breathing effect
  (bind (_direction _camerazdisp) (`Timeline|Timeline_0`)
    (:`Update`
      (`SceneComponent.K2_AddRelativeLocation` (`self.m_pCamera`) (`KismetMathLibrary.MakeVector` 0.0 0.0 (* _camerazdisp 0.02)) false false))))

(event `self.OnFootstep`
  ;[1 1 1] Surface sounds
  (bind (_bvalidhit _surface) (`self.GetSurfaceTypeBeneath`))
  (if _bvalidhit
    (`self.PlaySurfaceSoundWalking` _surface)))

(event `InputAxis|MoveForward` :consume false :overrideparent false
  (params (AxisValue :type "Float (single-precision)"))
  ;[1 1 1] CameraShakes
  (`self.CameraShakesPlay` AxisValue))

(event `InputAxis|MoveRight` :consume false :overrideparent false
  (params (AxisValue :type "Float (single-precision)"))
  ;[1 1 1] CameraShakes
  (`self.CameraShakesPlay` AxisValue))

(event `self.OnCharLanded`
  (`|ExecutionSequence`
    (:`then_0`
      ;[1 1 1] Surface sound
      (bind (_bvalidhit _surface) (`self.GetSurfaceTypeBeneath`))
      (if _bvalidhit
        (switch `EPhysicalSurface` _surface
          (:`SurfaceType_Default`
            (`GameplayStatics.PlaySound2D` "/Game/Sound/SFX/Player/player_1_land_sandgrass.player_1_land_sandgrass" 1.0 1.0 0.0 null null :!label _label))
          (:`SurfaceType1`
            (goto _label))
          (:`SurfaceType2`
            (`GameplayStatics.PlaySound2D` "/Game/Sound/SFX/Player/player_1_land_wood.player_1_land_wood" 1.0 1.0 0.0 null null)))))
    (:`then_1`
      (`PlayerController.ClientPlayCameraAnim` :`self` (`GameplayStatics.GetPlayerController` 0) :`AnimToPlay` "/Game/Player/Land_CAnim.Land_CAnim"))))

(event `self.OnJumped`
  ;[1 1 1] Sound
  (`GameplayStatics.PlaySound2D` "/Game/Sound/SFX/Player/player_1_jump_1.player_1_jump_1" 1.0 1.0 0.0 null null)
  (`PlayerController.ClientPlayCameraAnim` :`self` (`GameplayStatics.GetPlayerController` 0) :`AnimToPlay` "/Game/Player/Jump_CAnim.Jump_CAnim"))

(fn `CameraShakesPlay`
  (params (Scale :type "Float (double-precision)"))
  (switch `EMovementMode` (`CharacterMovementComponent.MovementMode` (`self.CharacterMovement`))
    (:`MOVE_Walking`
      _)
    (:`MOVE_NavWalking`
      _))
  (`PlayerController.ClientStartCameraShake` :`self` (`GameplayStatics.GetPlayerController` 0) :`Shake` "/Game/Player/CameraShake_Walk.CameraShake_Walk_C" :`Scale` Scale))

(fn `GetSurfaceTypeBeneath`
  (returns (bValidHit :type Boolean) (Surface :type "EPhysicalSurface Enum"))
  (bind _returnvalue (`self.K2_GetActorLocation`))
  (bind (_outhit _returnvalue_2) (`KismetSystemLibrary.LineTraceSingle` _returnvalue (- _returnvalue (`KismetMathLibrary.MakeVector` 0.0 0.0 (+ (`CapsuleComponent.CapsuleHalfHeight` (`self.CapsuleComponent`)) 20.0))) "TraceTypeQuery1"))
  (return _returnvalue_2 (`GameplayStatics.GetSurfaceType` _outhit)))

(fn `PlaySurfaceSoundWalking`
  (params (SurfaceType :type "EPhysicalSurface Enum" :default "SurfaceType_Default"))
  (locals (LoadedObject :type "Object Object Reference"))
  (switch `EPhysicalSurface` SurfaceType
    (:`SurfaceType_Default`
      (set `local.LoadedObject` (`self.SampleObjectLibrary` (`self.FootstepsLibrary_Soil`) 16) :!label _label))
    (:`SurfaceType1`
      (set `local.LoadedObject` (`self.SampleObjectLibrary` (`self.FootstepLibrary_Sand`) 16)))
    (:`SurfaceType2`
      (set `local.LoadedObject` (`self.SampleObjectLibrary` (`self.FootstepLibrary_Wood`) 16)))
    (:`SurfaceType4`
      (goto _label)))
  (bind _assound_wave (cast `SoundWave` (`local.LoadedObject`)))
  (`GameplayStatics.PlaySoundAtLocation` _assound_wave (`self.K2_GetActorLocation`) (struct) 1.0 1.0 0.0 null null self))

(fn `SampleObjectLibrary`
  (params (LibPath :type "SoftObjectPath Structure") (LibSize :type Integer))
  (returns (LoadedObject :type "Object Object Reference"))
  (bind _returnvalue (`ASTBlueprintLib.LoadObjectLibraryAssetAt` (`KismetMathLibrary.RandomInteger` LibSize) (`KismetSystemLibrary.BreakSoftObjectPath` LibPath)))
  (return _returnvalue))

(fn `ScaleVec4`
  (params (InVec :type "Vector4 Structure") (scale :type "Float (double-precision)" :default 1.0))
  (returns (OutVec :type "Vector4 Structure"))
  (bind (_x _y _z _w) (`KismetMathLibrary.BreakVector4` InVec))
  (return (`KismetMathLibrary.MakeVector4` (* scale _x) (* scale _y) (* scale _z) (* scale _w))))

(fn `UserConstructionScript`)