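; NarratorTrigger_BP is a box trigger that plays a narrator dialogue wave to the player on overlap.
; It fires only when the game instance's Canyon and Mine completion states match its configured flags, optionally just once.
; The spawned 2D dialogue is passed to ASTGamemode through NotifyNewDialogue.
; Save and load events persist the played state in the savegame's narrator map, keyed by the dialogue wave's path.
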(event `self.Box.OnComponentBeginOverlap`
  (params (OverlappedComponent :type "PrimitiveComponent Object Reference") (OtherActor :type "Actor Object Reference") (OtherComp :type "PrimitiveComponent Object Reference") (OtherBodyIndex :type Integer) (bFromSweep :type Boolean) (SweepResult :type "HitResult Structure (by ref)"))
  (`|ExecutionSequence`
    (:`then_0`
      (bind _asastgame_instance (cast `ASTGameInstance` (`GameplayStatics.GetGameInstance`))))
    (:`then_1`
      (if (and (== (`self.bWhenCanyonCompleted`) (`ASTGameInstance.IsCanyonLevelDone` _asastgame_instance)) (== (`ASTGameInstance.IsMineLevelDone` _asastgame_instance) (`self.bWhenMineCompleted`)))
        (if (`self.bPlayOnce`)
          (if (not (`self.bHasPlayedOnce`))
            (set `self.bHasPlayedOnce` true)
            (bind _returnvalue (`GameplayStatics.SpawnDialogue2D` (`self.Dialogue Wave`) (`self.NarratorToPlayer`) :!label _label))
            (bind _asastgamemode (cast `/Game/Misc/ASTGamemode` (`GameplayStatics.GetGameMode`)))
            (`/Game/Misc/ASTGamemode.NotifyNewDialogue` _asastgamemode _returnvalue))
          (else
            (goto _label)))))))

(event `self.OnSaveGame`
  (params (pSavegame :type "ASTSaveGame Object Reference"))
  (`BlueprintMapLibrary.Map_Add` (`ASTSaveGame.m_NarratorMap` pSavegame) (`KismetSystemLibrary.GetPathName` (`self.Dialogue Wave`)) (`self.bHasPlayedOnce`)))

(event `self.OnLoadGame`
  (params (pSavegame :type "ASTSaveGame Object Reference"))
  (bind _returnvalue (`KismetSystemLibrary.GetPathName` (`self.Dialogue Wave`)))
  (bind (_value _returnvalue_2) (`BlueprintMapLibrary.Map_Find` (`ASTSaveGame.m_NarratorMap` pSavegame) _returnvalue))
  (if _returnvalue_2
    (set `self.bHasPlayedOnce` _value)
    (else
      (`KismetSystemLibrary.PrintString` (`KismetStringLibrary.Concat_StrStr` "ERROR, could not load saved state for dialogue wave:\\n" _returnvalue)))))

(fn `UserConstructionScript`)